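; Barrel actor that plays metal impact sounds scaled by how hard it hits in physics collisions.
; On Hit, the normal impulse magnitude is normalized and fed into three float curves.
; Each curve sets the volume of its own attached sound, layering two medium impacts and one heavy impact by force.
; A DoOnce reset after a short delay throttles repeated hits.
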(event EventHit
  (params (MyComp :type Primitive%20Component%20Object%20Reference) (Other :type Actor%20Object%20Reference) (OtherComp :type Primitive%20Component%20Object%20Reference) (bSelfMoved :type Boolean) (HitLocation :type Vector :default "0, 0, 0") (HitNormal :type Vector :default "0, 0, 0") (NormalImpulse :type Vector :default "0, 0, 0") (Hit :type Hit%20Result%20Structure%20%28by%20ref%29))
  (bind _returnvalue (Math|Vector|VectorLength NormalImpulse))
  (bind _returnvalue_2 (Math|Float|NormalizetoRange _returnvalue 0.0 5e+05))
  (Utilities|FlowControl|DoOnce false :!label _label
    (:Completed
      (bind _returnvalue_3 (Class|GameplayStatics|PlaySoundAttached "/Game/Audio/SFX/COLLISION_impact_metal_medium_05.COLLISION_impact_metal_medium_05" MyComp))
      (Audio|Components|Audio|SetVolumeMultiplier _returnvalue_3 (Math|Curves|GetFloatValue (Variables|Default|GetPhysics_Curve_01) _returnvalue_2) :!class /Script/Engine.AudioComponent)
      (bind _returnvalue_4 (Class|GameplayStatics|PlaySoundAttached "/Game/Audio/SFX/COLLISION_impact_metal_medium_13.COLLISION_impact_metal_medium_13" MyComp))
      (Audio|Components|Audio|SetVolumeMultiplier _returnvalue_4 (Math|Curves|GetFloatValue (Variables|Default|GetPhysics_Curve_02) _returnvalue_2) :!class /Script/Engine.AudioComponent)
      (bind _returnvalue_5 (Class|GameplayStatics|PlaySoundAttached "/Game/Audio/SFX/COLLISION_impact_metal_heavy_01.COLLISION_impact_metal_heavy_01" MyComp))
      (Audio|Components|Audio|SetVolumeMultiplier _returnvalue_5 (Math|Curves|GetFloatValue (Variables|Default|GetPhysics_Curve_03) _returnvalue_2) :!class /Script/Engine.AudioComponent)
      (Utilities|FlowControl|Delay 0.1)
      (Utilities|FlowControl|Sequence
        (:then_0
          (goto _label Reset))))))

(fn ConstructionScript)