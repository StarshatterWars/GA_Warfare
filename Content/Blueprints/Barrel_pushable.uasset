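; Pushable barrel Blueprint that plays impact and rolling sounds from physics hits, with volume scaled by normalized impulse strength.
; Strong hits play a metal impact; weak hits increment a counter, also playing impacts until the count passes a threshold that starts the roll sound.
; A DoOnce blocks overlapping rolls until audio finishes, while a retriggerable delay resets the count and fades the roll once weak hits stop.
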(event Custom|OnAudioFinished_Event_0
  (Utilities|FlowControl|DoOnce false) ; enters at Reset
)

(event Collision|EventHit
  (params (MyComp :type Primitive%20Component%20Object%20Reference) (Other :type Actor%20Object%20Reference) (OtherComp :type Primitive%20Component%20Object%20Reference) (bSelfMoved :type Boolean) (HitLocation :type Vector :default "0, 0, 0") (HitNormal :type Vector :default "0, 0, 0") (NormalImpulse :type Vector :default "0, 0, 0") (Hit :type Hit%20Result%20Structure%20%28by%20ref%29))
  (bind _returnvalue (Math|Vector|VectorLength NormalImpulse))
  (bind _returnvalue_2 (Math|Float|NormalizetoRange _returnvalue 0.0 5e+05))
  (if (> _returnvalue_2 0.1)
    (bind _returnvalue_3 (Audio|SpawnSoundAttached "/Game/Audio/SFX/COLLISION_impact_metal_hard_11.COLLISION_impact_metal_hard_11" MyComp :!label _label))
    (Utilities|IsValid _returnvalue_3
      (:Is%20Valid
        (Audio|Components|Audio|SetVolumeMultiplier _returnvalue_3 _returnvalue_2 :!class /Script/Engine.AudioComponent)))
    (else
      (Utilities|FlowControl|Sequence
        (:then_0
          (Variables|Default|SetHitCount (+ (Variables|Default|GetHitCount) 1))
          (if (> (Variables|Default|GetHitCount) 4)
            (Utilities|FlowControl|DoOnce false
              (:Completed
                (bind _returnvalue_4 (Audio|SpawnSoundAttached "/Game/Audio/SFX/Barrel_Roll_PH.Barrel_Roll_PH" MyComp))
                (Utilities|IsValid _returnvalue_4
                  (:Is%20Valid
                    (Audio|Components|Audio|SetVolumeMultiplier _returnvalue_4 _returnvalue_2 :!class /Script/Engine.AudioComponent)
                    (EventDispatchers|AssignOnAudioFinished _returnvalue_4 (delegate Custom|OnAudioFinished_Event_0))))))
            (else
              (goto _label))))
        (:then_1
          (Utilities|FlowControl|RetriggerableDelay 0.2) ; Reset frequency
          (Variables|Default|SetHitCount 0)
          (Utilities|IsValid _returnvalue_4
            (:Is%20Valid
              (Audio|Components|Audio|FadeOut _returnvalue_4 0.3 0.0 :!class /Script/Engine.AudioComponent))))))))

(fn ConstructionScript)