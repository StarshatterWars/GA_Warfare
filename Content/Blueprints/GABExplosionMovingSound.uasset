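; Explosion actor that, when activated, fires a particle burst with a core sound and launches moving sound sources outward.
; It first aligns its yaw to the player-to-explosion line, so the sound layout is relative to the player's position.
; It spawns four projectile-driven emitters with attached sounds: an opposed left/right perpendicular pair and a swoosh pair spread around a 90-degree yaw offset, each pair with its own speed.
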(event Custom|Activate
  (bind _returnvalue (Transformation|GetActorRotation))
  (bind _returnvalue_2 (Transformation|GetActorRotation))
  (bind _particlesystem1 (Variables|Default|GetParticleSystem1))
  (bind _perpendicularspeed (Variables|Sound|GetPerpendicularSpeed))
  (bind _perpendicularspeed_2 (Variables|Sound|GetPerpendicularSpeed))
  (bind _swooshspread (Variables|Sound|GetSwooshSpread))
  (bind _swooshspeed (Variables|Sound|GetSwooshSpeed))
  (bind _swooshspeed_2 (Variables|Sound|GetSwooshSpeed))
  (bind _yaw (Class|KismetMathLibrary|BreakRot _returnvalue))
  (bind _yaw_2 (Class|KismetMathLibrary|BreakRot _returnvalue_2))
  ;[1 1 1] Rotate actor to face player
  (Transformation|SetActorRotation (Class|KismetMathLibrary|MakeRot 0.0 (.Yaw (Class|KismetMathLibrary|BreakRot (Math|Rotator|FindLookatRotation (Transformation|GetActorLocation (Game|GetPlayerCharacter 0)) (Transformation|GetActorLocation)))) 0.0))
  ;[1 1 1] Toggle explosion emitter
  (Components|Activation|Activate _particlesystem1 false)
  (Class|GameplayStatics|PlaySoundAttached (Variables|Sound|GetExplosion_Core) _particlesystem1)
  ;[1 1 1] Perpendicular sounds
  (bind _returnvalue_3 (Game|SpawnActorfromClass "/Game/Blueprints/ExplosionMovingSoundEmitter.ExplosionMovingSoundEmitter_C" (Math|Transform|MakeTransform (Transformation|GetActorLocation) (Class|KismetMathLibrary|MakeRot 0.0 (+ _yaw 0.0) 0.0)) false 0))
  (Variables|/Script/Engine.ProjectileMovementComponent|SetInitialSpeed (Variables|/Game/Blueprints/ExplosionMovingSoundEmitter.ExplosionMovingSoundEmitter_C|GetProjectileMovement1 _returnvalue_3) _perpendicularspeed_2)
  (Variables|/Script/Engine.ProjectileMovementComponent|SetMaxSpeed (Variables|/Game/Blueprints/ExplosionMovingSoundEmitter.ExplosionMovingSoundEmitter_C|GetProjectileMovement1 _returnvalue_3) _perpendicularspeed_2)
  (Class|GameplayStatics|PlaySoundAttached (Variables|Sound|GetRightPerpendicular) (VehicleSound|GetRootComponent _returnvalue_3))
  (bind _returnvalue_4 (Game|SpawnActorfromClass "/Game/Blueprints/ExplosionMovingSoundEmitter.ExplosionMovingSoundEmitter_C" (Math|Transform|MakeTransform (Transformation|GetActorLocation) (Class|KismetMathLibrary|MakeRot 0.0 (- _yaw 1.8e+02) 0.0)) false 0))
  (Variables|/Script/Engine.ProjectileMovementComponent|SetInitialSpeed (Variables|/Game/Blueprints/ExplosionMovingSoundEmitter.ExplosionMovingSoundEmitter_C|GetProjectileMovement1 _returnvalue_4) _perpendicularspeed)
  (Variables|/Script/Engine.ProjectileMovementComponent|SetMaxSpeed (Variables|/Game/Blueprints/ExplosionMovingSoundEmitter.ExplosionMovingSoundEmitter_C|GetProjectileMovement1 _returnvalue_4) _perpendicularspeed)
  (Class|GameplayStatics|PlaySoundAttached (Variables|Sound|GetLeftPerpendicular) (VehicleSound|GetRootComponent _returnvalue_4))
  ;[1 1 1] Swoosh sounds
  (bind _returnvalue_5 (Game|SpawnActorfromClass "/Game/Blueprints/ExplosionMovingSoundEmitter.ExplosionMovingSoundEmitter_C" (Math|Transform|MakeTransform (Transformation|GetActorLocation) (Class|KismetMathLibrary|MakeRot 0.0 (+ _yaw_2 (+ 9e+01 _swooshspread)) 0.0)) false 0))
  (Variables|/Script/Engine.ProjectileMovementComponent|SetInitialSpeed (Variables|/Game/Blueprints/ExplosionMovingSoundEmitter.ExplosionMovingSoundEmitter_C|GetProjectileMovement1 _returnvalue_5) _swooshspeed_2)
  (Variables|/Script/Engine.ProjectileMovementComponent|SetMaxSpeed (Variables|/Game/Blueprints/ExplosionMovingSoundEmitter.ExplosionMovingSoundEmitter_C|GetProjectileMovement1 _returnvalue_5) _swooshspeed_2)
  (Class|GameplayStatics|PlaySoundAttached (Variables|Sound|GetLeftSwoosh) (VehicleSound|GetRootComponent _returnvalue_5))
  (bind _returnvalue_6 (Game|SpawnActorfromClass "/Game/Blueprints/ExplosionMovingSoundEmitter.ExplosionMovingSoundEmitter_C" (Math|Transform|MakeTransform (Transformation|GetActorLocation) (Class|KismetMathLibrary|MakeRot 0.0 (+ _yaw_2 (- 9e+01 _swooshspread)) 0.0)) false 0))
  (Variables|/Script/Engine.ProjectileMovementComponent|SetInitialSpeed (Variables|/Game/Blueprints/ExplosionMovingSoundEmitter.ExplosionMovingSoundEmitter_C|GetProjectileMovement1 _returnvalue_6) _swooshspeed)
  (Variables|/Script/Engine.ProjectileMovementComponent|SetMaxSpeed (Variables|/Game/Blueprints/ExplosionMovingSoundEmitter.ExplosionMovingSoundEmitter_C|GetProjectileMovement1 _returnvalue_6) _swooshspeed)
  (Class|GameplayStatics|PlaySoundAttached (Variables|Sound|GetRightSwoosh) (VehicleSound|GetRootComponent _returnvalue_6)))

(fn ConstructionScript)