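; Player-driven tank that moves, turns, cycles cameras and fires projectiles, with all input actions gated by an Active flag.
; Axis input offsets forward motion by delta time and adds yaw per call, scaling driving and turning sound volumes to input strength.
; E cycles three cameras through a looping MultiGate.
; Right mouse spawns a TankProjectile with sound ahead of and above the tank, rate-limited by a Gate reopened after FiringInterval.
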(event EventTick
  (params (DeltaSeconds :type Float%20%28single-precision%29))
  (Variables|Default|SetDeltaTime DeltaSeconds))

(event EventBeginPlay
  (Input|EnableInput (Game|GetPlayerController 0))
  (Class|GameplayStatics|PlaySoundAttached (Variables|Sound|GetBase%20Sound) (VehicleSound|GetRootComponent))
  (bind _returnvalue (Class|GameplayStatics|PlaySoundAttached (Variables|Sound|GetDrivingSound) (VehicleSound|GetRootComponent)))
  (bind _returnvalue_2 (Class|GameplayStatics|PlaySoundAttached (Variables|Sound|GetTurningSound) (VehicleSound|GetRootComponent))))

(event Input|AxisEvents|InputAxisMoveForward
  (params (AxisValue :type Float%20%28single-precision%29))
  (if (Variables|Default|GetActive)
    (Transformation|AddActorLocalOffset (Math|Vector|MakeVector (* (Variables|Default|GetDeltaTime) (* (Variables|Default|GetSpeed) AxisValue)) 0.0 0.0) false)
    (Audio|Components|Audio|SetVolumeMultiplier (stale EventBeginPlay _returnvalue) (Math|Float|Absolute(Float) AxisValue) :!class /Script/Engine.AudioComponent)))

(event Input|AxisEvents|InputAxisMoveRight
  (params (AxisValue :type Float%20%28single-precision%29))
  (bind _returnvalue (Transformation|GetActorRotation))
  (bind (_pitch _yaw _roll) (Class|KismetMathLibrary|BreakRot _returnvalue))
  (if (Variables|Default|GetActive)
    (Transformation|SetActorRotation (Class|KismetMathLibrary|MakeRot _pitch (+ (* AxisValue (Variables|Default|GetRotateSpeed)) _yaw) _roll))
    (Audio|Components|Audio|SetVolumeMultiplier (stale EventBeginPlay _returnvalue_2) (Math|Float|Absolute(Float) AxisValue) :!class /Script/Engine.AudioComponent)))

(event Input|MouseEvents|RightMouseButton
  (bind _returnvalue (Transformation|GetActorRotation))
  (bind _returnvalue_2 (Transformation|GetActorLocation))
  (bind _turretoffset (Variables|Default|GetTurretOffset))
  (bind _returnvalue_3 (Math|Vector|GetForwardVector _returnvalue))
  (bind _returnvalue_4 (* _returnvalue_3 _turretoffset))
  (bind _returnvalue_5 (+ _returnvalue_2 _returnvalue_4))
  (bind _returnvalue_6 (+ _returnvalue_5 "0, 0,275.000000"))
  ;[1 1 1] Firing
  (:Pressed
    (if (Variables|Default|GetActive)
      (Utilities|FlowControl|Gate false :!label _label
        (:Exit
          (Utilities|FlowControl|Sequence
            (:then_0
              (Game|SpawnActorfromClass "/Game/Blueprints/TankProjectile.TankProjectile_C" (Math|Transform|MakeTransform _returnvalue_6 _returnvalue) true 0 0)
              (Audio|PlaySoundatLocation (Variables|Default|GetFiringSound) _returnvalue_6)
              (Utilities|FlowControl|Delay (Variables|Default|GetFiringInterval))
              (goto _label Open))
            (:then_1
              (goto _label Close))))))))

(event Input|KeyboardEvents|E
  (bind _camera1 (Variables|Default|GetCamera1))
  (bind _camera2 (Variables|Default|GetCamera2))
  (bind _camera3 (Variables|Default|GetCamera3))
  (:Pressed
    (if (Variables|Default|GetActive)
      (Utilities|FlowControl|MultiGate false true -1
        (:Out%200
          (Components|Activation|SetActive _camera1 true false)
          (Components|Activation|SetActive _camera2 false false)
          (Components|Activation|SetActive _camera3 false false))
        (:Out%201
          (Components|Activation|SetActive _camera1 false false)
          (Components|Activation|SetActive _camera2 true false)
          (Components|Activation|SetActive _camera3 false false))
        (:Out%202
          (Components|Activation|SetActive _camera1 false false)
          (Components|Activation|SetActive _camera2 false false)
          (Components|Activation|SetActive _camera3 true false))))))

(fn ConstructionScript)