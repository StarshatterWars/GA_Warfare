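; VestPutDown is an overlap trigger that removes the player's vest by clearing HasVest on MyCharacter.
; When a MyCharacter overlaps Box1, it updates player 0's character, plays an attached sound and hides the actor.
; A Gate closes to block retriggering until a three-second delay ends, then the actor reappears and the Gate reopens.
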(event OnComponentBeginOverlap(Box1)
  (params (OtherActor :type Actor%20Object%20Reference) (OtherComp :type Primitive%20Component%20Object%20Reference) (OtherBodyIndex :type Integer) (bFromSweep :type Boolean) (SweepResult :type Hit%20Result%20Structure%20%28by%20ref%29))
  (Utilities|FlowControl|Gate false :!label _label
    (:Exit
      (if (== (Utilities|GetClass OtherActor) "/Game/Blueprints/MyCharacter.MyCharacter_C")
        (bind _asmy_character (Utilities|Casting|CastToMyCharacter (Game|GetPlayerCharacter 0)))
        (Variables|/Game/Blueprints/MyCharacter.MyCharacter_C|SetHasVest _asmy_character false)
        (Class|GameplayStatics|PlaySoundAttached "/Engine/EditorSounds/Notifications/CompileFailed.CompileFailed" (VehicleSound|GetRootComponent))
        (Rendering|SetActorHiddenInGame true)
        (Utilities|FlowControl|Sequence
          (:then_0
            (goto _label Close))
          (:then_1
            (Utilities|FlowControl|Delay 3.0)
            (Rendering|SetActorHiddenInGame false)
            (goto _label Open)))))))

(fn ConstructionScript)