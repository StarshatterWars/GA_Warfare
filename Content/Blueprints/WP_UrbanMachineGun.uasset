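; Urban machine gun weapon that fires automatically from its Fire event until Release is called.
; Fire opens a gate that loops on a short delay, playing an attached sound and spawning a MyProjectile_backup each pass.
; Projectiles spawn at the gun's location plus an offset, both offset and aim following player 0's control rotation.
; Ammo check and decrement nodes exist but are disconnected, so ammo is unlimited.
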(event Custom|Release
  (bind _returnvalue (Game|Player|GetPlayerPawn 0))
  (bind _returnvalue_2 (Pawn|GetControlRotation _returnvalue :!class /Script/Engine.Pawn))
  (Utilities|FlowControl|Gate true) ; enters at Close
)

(event Custom|Fire
  (bind _returnvalue (Game|Player|GetPlayerPawn 0))
  (bind _returnvalue_2 (Pawn|GetControlRotation _returnvalue :!class /Script/Engine.Pawn))
  (Utilities|FlowControl|Sequence
    (:then_0
      (goto _label Open))
    (:then_1
      (Utilities|FlowControl|Gate true :!label _label
        (:Exit
          (Audio|SpawnSoundAttached "/Game/Audio/UrbanRetriggered.UrbanRetriggered" (VehicleSound|GetRootComponent))
          (Game|SpawnActorfromClass "/Game/Blueprints/MyProjectile_backup.MyProjectile_backup_C" (Math|Transform|MakeTransform (+ (Transformation|GetActorLocation) (Math|Vector|RotateVector (Variables|Default|GetGunOffset) _returnvalue_2)) _returnvalue_2) "AlwaysSpawn" 0 0)
          (Utilities|FlowControl|Delay 0.1)
          (goto _label))))))

(fn ConstructionScript)