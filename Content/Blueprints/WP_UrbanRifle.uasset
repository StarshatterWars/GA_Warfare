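; Urban rifle weapon Blueprint that fires a projectile along the first player's control rotation.
; Fire plays an attached sniper sound and spawns MyProjectile_backup at the weapon's location plus a rotated gun offset, even if colliding.
; A DoOnce that resets after a short delay limits the fire rate.
; An AmmoCount check exists but is disconnected, so ammo does not restrict firing.
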(event Custom|Fire
  (bind _returnvalue (Game|Player|GetPlayerPawn 0))
  (bind _returnvalue_2 (Pawn|GetControlRotation _returnvalue :!class /Script/Engine.Pawn))
  (Utilities|FlowControl|DoOnce false :!label _label
    (:Completed
      (Class|GameplayStatics|PlaySoundAttached "/Game/Audio/SFX/Sniper_UW.Sniper_UW" (VehicleSound|GetRootComponent))
      (Game|SpawnActorfromClass "/Game/Blueprints/MyProjectile_backup.MyProjectile_backup_C" (Math|Transform|MakeTransform (+ (Transformation|GetActorLocation) (Math|Vector|RotateVector (Variables|Default|GetGunOffset) _returnvalue_2)) _returnvalue_2) true 0 0)
      (Utilities|FlowControl|Delay 0.5)
      (goto _label Reset))))

(fn ConstructionScript)